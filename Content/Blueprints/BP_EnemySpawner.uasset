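; Enemy spawner that creates side-scrolling NPCs once something first overlaps its SpawnBox.
; A DoOnce-guarded overlap starts a Delay-paced loop that spawns at the box's location, records each NPC in EnemyList and repeats until the count reaches the maximum.
; Debug prints trace each pass, IsSpawning clears when the loop ends, and the EnemyDied event is an empty stub.
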(event `Start Spawning`
  (bind _max_spawn_amount (`self.Max Spawn Amount`))
  (bind _current_spawn_amount (`self.Current Spawn Amount`))
  (bind _returnvalue (< _current_spawn_amount _max_spawn_amount))
  (bind _returnvalue_2 (`|SpawnActorFromClass` "/Game/Variant_SideScroller/Blueprints/AI/BP_SideScrolling_NPC.BP_SideScrolling_NPC_C" (`KismetMathLibrary.MakeTransform` (`SceneComponent.K2_GetComponentLocation` (`self.Spawn Box`))) "Undefined" "MultiplyWithRoot" null null :!label _label))
  (`KismetSystemLibrary.PrintString` "Hello")
  (`KismetArrayLibrary.Array_Add` (`self.Enemy List`) _returnvalue_2)
  (`/Engine/EditorBlueprintResources/StandardMacros.IncrementInt` (`self.Current Spawn Amount`)
    (:`  `
      (`KismetSystemLibrary.Delay` (`self.Spawn Interval`))
      (`KismetSystemLibrary.PrintString` (`KismetStringLibrary.Concat_StrStr` "Max: " (`KismetStringLibrary.Conv_IntToString` _max_spawn_amount) "Current" (`KismetStringLibrary.Conv_IntToString` _current_spawn_amount)) true true (struct :`G` 0.66 :`B` 1.0 :`A` 1.0) 20.0)
      (`KismetSystemLibrary.PrintString` (`KismetStringLibrary.Conv_BoolToString` _returnvalue) true true (struct :`G` 0.66 :`B` 1.0 :`A` 1.0) 20.0)
      (if _returnvalue
        (goto _label)
        (else
          (set `self.Is Spawning` false))))))

(event `self.Spawn Box.OnComponentBeginOverlap`
  (params (OverlappedComponent :type "PrimitiveComponent Object Reference") (OtherActor :type "Actor Object Reference") (OtherComp :type "PrimitiveComponent Object Reference") (OtherBodyIndex :type Integer) (bFromSweep :type Boolean) (SweepResult :type "HitResult Structure (by ref)"))
  (`/Engine/EditorBlueprintResources/StandardMacros.DoOnce` false
    (:`Completed`
      (`self.Start Spawning`))))

(event `Enemy Died`)

(fn `UserConstructionScript`)